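; DoorBP is a double sliding door, apparently glass, that opens once when something overlaps its OpenDoorCollision component.
; The first overlap passes a DoOnce, plays an opening sound at the actor's location and starts both panels moving together.
; MoveComponentTo slides the left and right panels apart along local X by MoveDistance over one second, then each is hidden.
; It has no closing or reset logic.
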(event OnComponentBeginOverlap(OpenDoorCollision)
  (params (OverlappedComponent :type Primitive%20Component%20Object%20Reference) (OtherActor :type Actor%20Object%20Reference) (OtherComp :type Primitive%20Component%20Object%20Reference) (OtherBodyIndex :type Integer) (bFromSweep :type Boolean) (SweepResult :type Hit%20Result%20Structure%20%28by%20ref%29))
  (bind _leftdoor (Variables|Default|GetLeftDoor))
  (bind _rightdoor (Variables|Default|GetRightDoor))
  (bind _relativelocation (Variables|/Script/Engine.SceneComponent|GetRelativeLocation _rightdoor))
  (bind _relativelocation_2 (Variables|/Script/Engine.SceneComponent|GetRelativeLocation _leftdoor))
  (Utilities|FlowControl|DoOnce false
    (:Completed
      (Audio|PlaySoundatLocation "/Game/BPs/Doors_Glass/DoorOpening.DoorOpening" (Transformation|GetActorLocation) "0, 0, 0" 1.0 1.0 0.0 0 0 0)
      (Utilities|FlowControl|Sequence
        (:then_0
          ;[1 1 1] Open Left Door
          (Components|MoveComponentTo _leftdoor (Math|Vector|MakeVector (- (.x _relativelocation_2) (Variables|Default|GetMoveDistance)) (.y _relativelocation_2) (.z _relativelocation_2)) (Variables|/Script/Engine.SceneComponent|GetRelativeRotation _leftdoor) false false 1.0 false)
          (Rendering|SetVisibility _leftdoor false false))
        (:then_1
          ;[1 1 1] Open Right Door
          (Components|MoveComponentTo _rightdoor (Math|Vector|MakeVector (+ (Variables|Default|GetMoveDistance) (.x _relativelocation)) (.y _relativelocation) (.z _relativelocation)) (Variables|/Script/Engine.SceneComponent|GetRelativeRotation _rightdoor) false false 1.0 false)
          (Rendering|SetVisibility _rightdoor false false))))))

(fn ConstructionScript)