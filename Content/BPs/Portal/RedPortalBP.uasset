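; RedPortalBP is a portal that fades in, spawns a series of Alpha_Red actors at its arrow, then fades out and destroys itself.
; Timelines drive the Fade parameter on a dynamic red portal material, with an attenuated portal sound that fades alongside the closing.
; A delayed loop spawns up to a configurable count, storing each actor in an array that the DestroySpawnedActors event can clear from the world.
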(event Custom|DestroySpawnedActors
  (for _array_element (Variables|Default|GetArrayOfAlpha)
    (Actor|DestroyActor _array_element)))

(event EventBeginPlay
  (bind _arrow (Variables|Default|GetArrow))
  ;[1 1 1] Fade In Material
  (bind _returnvalue (Audio|SpawnSoundatLocation "/Game/BPs/Portal/Portal.Portal" (Transformation|GetActorLocation) "0, 0, 0" 0.3 1.0 0.0 (Variables|Default|GetSpawnPortalAttenuation) 0))
  (Variables|Default|SetPortalSound _returnvalue)
  (bind _returnvalue_2 (Rendering|Material|CreateDynamicMaterialInstance (Variables|Default|GetParticleSystem) 0 "/Game/BPs/Portal/ParticleNMaterial/M_Portal_InstRed.M_Portal_InstRed" "None" :!class /Script/Engine.PrimitiveComponent))
  (bind _output_get (Variables|Default|SetMaterialRef _returnvalue_2))
  (bind _fade (Timeline|FadePortal Play) ; FadePortal
    (:Update
      (Rendering|Material|SetScalarParameterValue _output_get "Fade" (Math|Float|Lerp -1.0 0.0 _fade) :!class /Script/Engine.MaterialInstanceDynamic))
    (:Finished
      ;[1 1 1] Spawn Alphas
      (Variables|Default|SetAlphaCounter 0)
      (bind _returnvalue_3 (Game|SpawnActorfromClass "/Game/Alpha/Alpha_Red.Alpha_Red_C" (Math|Transform|MakeTransform (Transformation|GetWorldLocation _arrow) (Transformation|GetWorldRotation _arrow)) "AlwaysSpawn" 0 0 :!label _label))
      (bind _output_get_2 (Variables|Default|SetAlphaRef _returnvalue_3))
      (Utilities|Array|Add (Variables|Default|GetArrayOfAlpha) _output_get_2)
      (Variables|Default|SetArrayOfAlpha (Variables|Default|GetArrayOfAlpha))
      (bind _result (Math|Integer|IncrementInt (Variables|Default|GetAlphaCounter))
        (:%20%20
          (Variables|Default|SetAlphaCounter _result)
          (Audio|PlaySound2D "/Game/BPs/Portal/SpawnedAlpha.SpawnedAlpha" 0.2 1.0 0.0 0 0)
          (if (>= (Variables|Default|GetAlphaCounter) (Variables|Default|GetAlphaCounterMax))
            ;[1 1 1] Fade Out Material
            (Audio|Components|Audio|FadeOut (Variables|Default|GetPortalSound) 3.0 0.0 "Linear" :!class /Script/Engine.AudioComponent)
            (bind _fade_2 (Timeline|FadePortalReverse Play)
              (:Update
                (Rendering|Material|SetScalarParameterValue (Variables|Default|GetMaterialRef) "Fade" (Math|Float|Lerp 0.0 -1.0 _fade_2) :!class /Script/Engine.MaterialInstanceDynamic))
              (:Finished
                (Actor|DestroyActor)))
            (else
              (Utilities|FlowControl|Delay (Variables|Default|GetSpawnAlphaDelay))
              (goto _label))))))))

(fn ConstructionScript)