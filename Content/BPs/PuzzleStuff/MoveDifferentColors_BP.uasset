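; MoveDifferentColors_BP is a puzzle switch that raises and lowers colored platforms when a red or blue tracer hits its box.
; Hits only count while the referenced Laser's CanMovable is true, and the tracer's class selects the color.
; Red tracers toggle RedMovable, while blue tracers toggle BlueMovable and GroundMovable together.
; A boolean per color alternates the Up and Down messages sent to those platforms.
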(event OnComponentHit(Box)
  (params (HitComponent :type Primitive%20Component%20Object%20Reference) (OtherActor :type Actor%20Object%20Reference) (OtherComp :type Primitive%20Component%20Object%20Reference) (NormalImpulse :type Vector :default "0, 0, 0") (Hit :type Hit%20Result%20Structure%20%28by%20ref%29))
  (bind _redmovable (Variables|Default|GetRedMovable))
  (bind _bluemovable (Variables|Default|GetBlueMovable))
  (bind _groundmovable (Variables|Default|GetGroundMovable))
  (if (Variables|/Game/BPs/PuzzleStuff/LaserForPuzzle_BP.LaserForPuzzle_BP_C|GetCanMovable? (Variables|Default|GetLaser))
    (Utilities|Casting|CastToTracer_RedBP OtherActor
      (:then
        ;[1 1 1] Move Red Platform
        (if (Variables|Default|GetUp?Red)
          (Class|InterfaceforPlatforms|Down(Message) _redmovable)
          (Variables|Default|SetUp?Red false)
          (else
            (Class|InterfaceforPlatforms|Up(Message) _redmovable)
            (Variables|Default|SetUp?Red true))))
      (:CastFailed
        (Utilities|Casting|CastToTracer_BlueBP OtherActor)
        ;[1 1 1] Move Blue Platform
        (if (Variables|Default|GetUp?Blue)
          (Class|InterfaceforPlatforms|Down(Message) _bluemovable)
          (Class|InterfaceforPlatforms|Down(Message) _groundmovable)
          (Variables|Default|SetUp?Blue false)
          (else
            (Class|InterfaceforPlatforms|Up(Message) _bluemovable)
            (Class|InterfaceforPlatforms|Up(Message) _groundmovable)
            (Variables|Default|SetUp?Blue true)))))))

(fn ConstructionScript)