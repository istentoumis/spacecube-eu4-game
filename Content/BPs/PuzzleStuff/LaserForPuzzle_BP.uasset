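; Puzzle laser that casts a red or blue beam, kills the player on contact and signals a linked actor's door to open or close.
; LookIfCubeCollides uses gated line traces to detect the player's cube, comparing its border color to the beam's.
; A match shortens the beam to the cube, clears CanMovable and opens the door.
; The trigger box rescales with beam length, and ChangeColor toggles the beam's material color.
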(event OnComponentBeginOverlap(Box)
  (params (OverlappedComponent :type Primitive%20Component%20Object%20Reference) (OtherActor :type Actor%20Object%20Reference) (OtherComp :type Primitive%20Component%20Object%20Reference) (OtherBodyIndex :type Integer) (bFromSweep :type Boolean) (SweepResult :type Hit%20Result%20Structure%20%28by%20ref%29))
  ;[1 1 1] Player collide with Laser
  (bind _asfirst_person_character_bp (Utilities|Casting|CastToFirstPersonCharacter_BP OtherActor))
  (Utilities|FlowControl|DoOnce false :!label _label
    (:Completed
      (Utilities|Time|PauseTimerbyHandle (Variables|Default|GetTimerHandle))
      (Input|DisableInput _asfirst_person_character_bp (Game|GetPlayerController 0))
      (Viewport|RemoveAllWidgets)
      (bind _returnvalue (UserInterface|CreateWidget "/Game/BPs/Laser/DeathByLaser_WB.DeathByLaser_WB_C"))
      (UserInterface|Viewport|AddtoViewport _returnvalue 0)
      (bind _returnvalue_2 (Audio|SpawnSound2D "/Game/BPs/Laser/Sparks/CubeSparksEffect.CubeSparksEffect" 1.0 1.0 0.0 0))
      (Utilities|FlowControl|Delay 2.0)
      (Components|DestroyComponent _returnvalue_2)
      (CameraFades|StartCameraFade :self (Game|GetPlayerCameraManager 0) :FromAlpha 1.0 :Duration 1.0 :bHoldWhenFinished true)
      (Widget|RemovefromParent _returnvalue)
      (Actor|DestroyActor _asfirst_person_character_bp)
      (goto _label Reset))))

(event Custom|LookIfCubeCollides
  (bind _returnvalue (Game|GetPlayerCharacter 0))
  (bind _returnvalue_2 (Game|GetPlayerCharacter 0))
  (bind _laserstartpoint (Variables|Default|GetLaserStartPoint))
  (bind _defaultbeamendpoint (Variables|Default|GetDefaultBeamEndPoint))
  (bind _actor (Variables|Default|GetActor))
  (bind _laserbeam (Variables|Default|GetLaserBeam))
  (bind _asfirst_person_character_bp (Utilities|Casting|CastToFirstPersonCharacter_BP _returnvalue_2))
  (bind _asfirst_person_character_bp_2 (Utilities|Casting|CastToFirstPersonCharacter_BP _returnvalue))
  (bind _cube (Variables|/Game/FirstPersonCharacter/FirstPersonCharacter_BP.FirstPersonCharacter_BP_C|GetCube _asfirst_person_character_bp_2))
  (bind _cube_2 (Variables|/Game/FirstPersonCharacter/FirstPersonCharacter_BP.FirstPersonCharacter_BP_C|GetCube _asfirst_person_character_bp))
  ;[1 1 1] Check if Cube is alive, his height and if its color changed
  (if (Variables|/Game/FirstPersonCharacter/FirstPersonCharacter_BP.FirstPersonCharacter_BP_C|GetCubeisAlive? _asfirst_person_character_bp)
    (bind _returnvalue_3 (Rendering|Material|GetScalarParameterValue (Variables|/Game/BPs/Cube/Cube.Cube_C|GetDynamicMaterialInst _cube_2) "Max" :!class /Script/Engine.MaterialInstanceDynamic))
    (if (== _returnvalue_3 14.0)
      (Utilities|FlowControl|Sequence
        (:then_0
          (Utilities|FlowControl|Sequence
            (:then_0
              (if (Variables|/Game/BPs/Cube/Cube.Cube_C|GetColorChanged? _cube_2)
                (Utilities|FlowControl|DoOnce false :!label _label
                  (:Completed
                    _))
                (else
                  (Utilities|FlowControl|Sequence
                    (:then_0
                      ;[1 1 1] Spawn LineTrace for Beam
                      (Utilities|FlowControl|DoOnce false :!label _label_2
                        (:Completed
                          _)))
                    (:then_1
                      (goto _label_8 Reset))))))
            (:then_1
              (goto _label Reset))))
        (:then_1
          (if (== (.Z (Math|Vector|BreakVector (.Location (Math|Transform|BreakTransform (Transformation|GetRelativeTransform (Variables|/Game/BPs/PuzzleStuff/Platforms/UpNDownPlatform_BP.UpNDownPlatform_BP_C|GetStaticMesh (Variables|Default|GetPlatform))))))) 0.0)
            (Utilities|FlowControl|DoOnce false :!label _label_3
              (:Completed
                _))
            (else
              (goto _label_3 Reset)))))
      (bind _outhit (Collision|LineTraceByChannel (Transformation|GetWorldLocation (Variables|Default|GetLaserStartPoint)) (+ (Transformation|GetWorldLocation _laserstartpoint) (* (Math|Vector|GetForwardVector _laserstartpoint) 1e+04)) "TraceTypeQuery1" false 0 "None"))
      ;[1 1 1] Check if the Trace hit the cube
      (if (== (.HitActor (Collision|BreakHitResult _outhit)) _cube)
        ;[1 1 1] Check if the beam has the same color as the cube
        (bind _returnvalue_4 (Rendering|Material|GetVectorParameterValue (Variables|/Game/BPs/Cube/Cube.Cube_C|GetDynamicMaterialInst _cube) "Borders" :!class /Script/Engine.MaterialInstanceDynamic))
        (bind _returnvalue_5 (Rendering|Material|GetVectorParameterValue (Variables|Default|GetMaterialRef) "EmissiveColour" :!class /Script/Engine.MaterialInstanceDynamic))
        (if (== _returnvalue_4 _returnvalue_5)
          (Utilities|FlowControl|DoOnce false :!label _label_4
            (:Completed
              (Variables|Default|SetCanMovable? false)
              (Class|OpenPuzzleDoorInterface|OpenDoor(Message) _actor)
              (Utilities|FlowControl|Sequence
                (:then_0
                  ;[1 1 1] Beam collide with cube
                  (Transformation|SetWorldLocation (Variables|Default|GetSparks) (.Location (Collision|BreakHitResult _outhit)) false false)
                  (Transformation|SetWorldLocation (Variables|Default|GetSparksSound) (.Location (Collision|BreakHitResult _outhit)) false false)
                  (Class|ParticleSystemComponent|SetBeamEndPoint _laserbeam 0 (.Location (Collision|BreakHitResult _outhit)))
                  (CallFunction|ScaleTriggerBox (.Location (Collision|BreakHitResult _outhit)))
                  (Variables|/Game/BPs/Cube/Cube.Cube_C|SetColorChanged? _cube false :!label _label_5)
                  (goto _label Reset))
                (:then_1
                  (goto _label_6 Reset)))))
          (else
            (Utilities|FlowControl|DoOnce false :!label _label_6
              (:Completed
                (Variables|Default|SetCanMovable? true)
                (Class|OpenPuzzleDoorInterface|CloseDoor(Message) _actor)
                (Utilities|FlowControl|Sequence
                  (:then_0
                    (Utilities|FlowControl|Sequence
                      (:then_0
                        ;[1 1 1] If not colliding only Sparks/Sound to Cube for Style
                        (Transformation|SetWorldLocation (Variables|Default|GetSparks) (.Location (Collision|BreakHitResult _outhit)) false false)
                        (Transformation|SetWorldLocation (Variables|Default|GetSparksSound) (.Location (Collision|BreakHitResult _outhit)) false false)
                        ;[1 1 1] Default Beam Location
                        (Class|ParticleSystemComponent|SetBeamEndPoint _laserbeam 0 _defaultbeamendpoint :!label _label_7)
                        (CallFunction|ScaleTriggerBox _defaultbeamendpoint))
                      (:then_1
                        (goto _label_5))))
                  (:then_1
                    (goto _label_4 Reset))))))))
      (else
        (Utilities|FlowControl|Sequence
          (:then_0
            (goto _label_2 Reset))
          (:then_1
            (Utilities|FlowControl|DoOnce false :!label _label_8
              (:Completed
                (Variables|Default|SetCanMovable? true)
                (Utilities|FlowControl|Sequence
                  (:then_0
                    (Class|OpenPuzzleDoorInterface|CloseDoor(Message) (Variables|Default|GetActor))
                    (Transformation|SetWorldLocation (Variables|Default|GetSparks) _defaultbeamendpoint false false)
                    (Transformation|SetWorldLocation (Variables|Default|GetSparksSound) _defaultbeamendpoint false false)
                    (goto _label_7))
                  (:then_1
                    (goto _label_4 Reset)))))))))
    (else
      (goto _label_8))))

(event EventChangeColor
  (bind _materialref (Variables|Default|GetMaterialRef))
  (bind _returnvalue (Rendering|Material|GetVectorParameterValue _materialref "EmissiveColour" :!class /Script/Engine.MaterialInstanceDynamic))
  (if (== _returnvalue "(R=1.000000,G=0.000000,B=0.000000,A=1.000000)")
    (Rendering|Material|SetVectorParameterValue _materialref "EmissiveColour" "(R=0.000000,G=0.000000,B=1.000000,A=1.000000)" :!class /Script/Engine.MaterialInstanceDynamic)
    (else
      (Rendering|Material|SetVectorParameterValue _materialref "EmissiveColour" "(R=1.000000,G=0.000000,B=0.000000,A=1.000000)" :!class /Script/Engine.MaterialInstanceDynamic))))

(event EventBeginPlay
  (bind _laserstartpoint (Variables|Default|GetLaserStartPoint))
  ;[1 1 1] Create Beam
  (bind (_outhit _returnvalue) (Collision|LineTraceByChannel (Transformation|GetWorldLocation (Variables|Default|GetLaserStartPoint)) (+ (Transformation|GetWorldLocation _laserstartpoint) (* (Math|Vector|GetForwardVector _laserstartpoint) 1e+04)) "TraceTypeQuery1" false 0 "None"))
  (if _returnvalue
    (bind _output_get (Variables|Default|SetDefaultBeamEndPoint (.Location (Collision|BreakHitResult _outhit))))
    (CallFunction|CreateBeam (Transformation|GetWorldLocation (Variables|Default|GetLaserStartPoint)) _output_get)
    (CallFunction|ScaleTriggerBox _output_get)
    (if (Variables|Default|GetisRed?)
      (CallFunction|SetMaterial/Sparks/SparksSoundRed)
      (else
        (CallFunction|SetMaterial/Sparks/SparksSoundBlue)))
    (bind _returnvalue_2 (Utilities|Time|SetTimerbyEvent (EventDispatchers|CreateEvent :!event Custom|LookIfCubeCollides) 0.05 true))
    (bind _output_get_2 (Variables|Default|SetTimerHandle _returnvalue_2))
    (Utilities|Time|PauseTimerbyHandle _output_get_2)))

(fn ConstructionScript)

(fn CreateBeam
  (params (StartPoint :type Vector) (EndPoint :type Vector))
  (bind _returnvalue (Effects|SpawnEmitteratLocation "/Game/BPs/Laser/LaserParticle/Laser_P.Laser_P" StartPoint))
  (bind _output_get (Variables|Default|SetLaserBeam _returnvalue))
  (Class|ParticleSystemComponent|SetBeamEndPoint _output_get 0 EndPoint))

(fn ScaleTriggerBox
  (params (EndLocation :type Vector))
  (bind _laserstartpoint (Variables|Default|GetLaserStartPoint))
  (bind _box (Variables|Default|GetBox))
  (bind _returnvalue (Transformation|GetWorldLocation _laserstartpoint))
  (bind _returnvalue_2 (- EndLocation _returnvalue))
  (bind _returnvalue_3 (Math|Vector|VectorLength _returnvalue_2))
  (bind _returnvalue_4 (/ _returnvalue_3 2.0))
  (Transformation|SetRelativeScale3D _box (Math|Vector|MakeVector _returnvalue_4 1.0 1.0))
  (Transformation|SetRelativeLocation _box (Math|Vector|MakeVector _returnvalue_4 0.0 0.0) false false))

(fn SetMaterial/Sparks/SparksSoundRed
  (bind _defaultbeamendpoint (Variables|Default|GetDefaultBeamEndPoint))
  (bind _returnvalue (Rendering|Material|CreateDynamicMaterialInstance "/Game/BPs/Laser/LaserParticle/LaserMaterial_Inst.LaserMaterial_Inst" "None" :!class /Script/Engine.KismetMaterialLibrary))
  (bind _output_get (Variables|Default|SetMaterialRef _returnvalue))
  (Rendering|Material|SetMaterial (Variables|Default|GetLaserBeam) 0 _output_get)
  (Rendering|Material|SetVectorParameterValue _output_get "EmissiveColour" "(R=1.000000,G=0.000000,B=0.000000,A=1.000000)" :!class /Script/Engine.MaterialInstanceDynamic)
  (bind _returnvalue_2 (Effects|SpawnEmitteratLocation "/Game/BPs/Laser/Sparks/P_WeldSparks_Red.P_WeldSparks_Red" _defaultbeamendpoint))
  (Variables|Default|SetSparks _returnvalue_2)
  (bind _returnvalue_3 (Audio|SpawnSoundatLocation "/Game/BPs/Laser/Sparks/CubeSparksEffect.CubeSparksEffect" _defaultbeamendpoint "0, 0, 0" 1.0 1.0 0.0 (Variables|Default|GetAttenuationSparks) 0))
  (Variables|Default|SetSparksSound _returnvalue_3))

(fn SetMaterial/Sparks/SparksSoundBlue
  (bind _defaultbeamendpoint (Variables|Default|GetDefaultBeamEndPoint))
  (bind _returnvalue (Rendering|Material|CreateDynamicMaterialInstance "/Game/BPs/Laser/LaserParticle/LaserMaterial_Inst.LaserMaterial_Inst" "None" :!class /Script/Engine.KismetMaterialLibrary))
  (bind _output_get (Variables|Default|SetMaterialRef _returnvalue))
  (Rendering|Material|SetMaterial (Variables|Default|GetLaserBeam) 0 _output_get)
  (Rendering|Material|SetVectorParameterValue _output_get "EmissiveColour" "(R=0.000000,G=0.000000,B=1.000000,A=1.000000)" :!class /Script/Engine.MaterialInstanceDynamic)
  (bind _returnvalue_2 (Effects|SpawnEmitteratLocation "/Game/BPs/Laser/Sparks/P_WeldSparks_Blue.P_WeldSparks_Blue" _defaultbeamendpoint))
  (Variables|Default|SetSparks _returnvalue_2)
  (bind _returnvalue_3 (Audio|SpawnSoundatLocation "/Game/BPs/Laser/Sparks/CubeSparksEffect.CubeSparksEffect" _defaultbeamendpoint "0, 0, 0" 1.0 1.0 0.0 (Variables|Default|GetAttenuationSparks) 0))
  (Variables|Default|SetSparksSound _returnvalue_3))