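; A puzzle platform Blueprint that slides back and forth along its local Y axis.
; Up and Down events play and reverse a timeline whose Movement track, scaled by MovementSpeed, sets the mesh's relative location.
; A hit from the first-person character plays a landing sound.
; At BeginPlay, platforms not flagged IsRed swap to an alternate material.
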(event OnComponentHit(StaticMesh)
  (params (HitComponent :type Primitive%20Component%20Object%20Reference) (OtherActor :type Actor%20Object%20Reference) (OtherComp :type Primitive%20Component%20Object%20Reference) (NormalImpulse :type Vector :default "0, 0, 0") (Hit :type Hit%20Result%20Structure%20%28by%20ref%29))
  (Utilities|Casting|CastToFirstPersonCharacter_BP OtherActor)
  (Audio|PlaySound2D "/Game/BPs/PuzzleStuff/Platforms/JumpOnPlat.JumpOnPlat" 1.0 1.0 0.0 0 0))

(event EventBeginPlay
  (if (not (Variables|Default|GetisRed?))
    (Rendering|Material|SetMaterial (Variables|Default|GetStaticMesh) 0 "/Game/BPs/PuzzleStuff/Platforms/PlatformMat_Inst1.PlatformMat_Inst1")))

(event EventUp
  (bind _movement (Timeline|Timeline_0 Play)
    (:Update
      (Transformation|SetRelativeLocation (Variables|Default|GetStaticMesh) (Math|Vector|MakeVector 0.0 (* _movement (Variables|Default|GetMovementSpeed)) 0.0) false false))))

(event EventDown
  (bind _movement (Timeline|Timeline_0 Reverse)
    (:Update
      (Transformation|SetRelativeLocation (Variables|Default|GetStaticMesh) (Math|Vector|MakeVector 0.0 (* _movement (Variables|Default|GetMovementSpeed)) 0.0) false false))))

(fn ConstructionScript)