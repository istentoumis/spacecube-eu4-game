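; Red or blue laser hazard that aims at the player and kills them when its trace reaches them.
; BeginPlay shows sensed and countdown widgets, then spawns the beam and starts a looping timer that retraces to the player, moving beam end, sparks and sound.
; The player's cube blocks only a beam of matching color; otherwise the trace ignores it.
; DoOnce-gated delays cycle the laser on and off; death triggers a fade and destroys the character.
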(event Custom|LookIfCubeCollides
  (bind _returnvalue (Game|GetPlayerCharacter 0))
  (bind _returnvalue_2 (Game|GetPlayerCharacter 0))
  (bind _asfirst_person_character_bp (Utilities|Casting|CastToFirstPersonCharacter_BP _returnvalue))
  (bind _asfirst_person_character_bp_2 (Utilities|Casting|CastToFirstPersonCharacter_BP _returnvalue_2))
  (bind _cube (Variables|/Game/FirstPersonCharacter/FirstPersonCharacter_BP.FirstPersonCharacter_BP_C|GetCube _asfirst_person_character_bp))
  (Utilities|FlowControl|Sequence
    (:then_0
      (if (Variables|/Game/FirstPersonCharacter/FirstPersonCharacter_BP.FirstPersonCharacter_BP_C|GetCubeisAlive? (.AsFirst%20Person%20Character%20BP (Utilities|Casting|CastToFirstPersonCharacter_BP (Game|GetPlayerCharacter 0))))
        ;[1 1 1] If cube's color!=beam's color then ignore CUBE
        (bind _returnvalue_3 (Rendering|Material|GetVectorParameterValue (Variables|/Game/BPs/Cube/Cube.Cube_C|GetDynamicMaterialInst _cube) "Borders" :!class /Script/Engine.MaterialInstanceDynamic))
        (bind _returnvalue_4 (Rendering|Material|GetVectorParameterValue (Variables|Default|GetMaterialRef) "EmissiveColour" :!class /Script/Engine.MaterialInstanceDynamic))
        (if (== _returnvalue_3 _returnvalue_4)
          ;[1 1 1] LineTrace blocks cube
          (bind _outhit (Collision|LineTraceForObjects (Transformation|GetWorldLocation (Variables|Default|GetLaserStartPoint)) (Transformation|GetActorLocation _asfirst_person_character_bp_2) (Variables|Default|GetObjectTypes) false 0 "None" :!label _label))
          (Transformation|SetWorldLocation (Variables|Default|GetSparks) (.Location (Collision|BreakHitResult _outhit)) false false)
          (Transformation|SetWorldLocation (Variables|Default|GetSparksSound) (.Location (Collision|BreakHitResult _outhit)) false false)
          (Class|ParticleSystemComponent|SetBeamEndPoint (Variables|Default|GetLaserBeam) 0 (.Location (Collision|BreakHitResult _outhit)))
          (if (== (.HitActor (Collision|BreakHitResult _outhit)) _asfirst_person_character_bp_2)
            ;[1 1 1] Player Dead
            (Utilities|FlowControl|DoOnce false :!label _label_2
              (:Completed
                (Variables|Default|SetStop? true)
                (bind _asfirst_person_character_bp_3 (Utilities|Casting|CastToFirstPersonCharacter_BP (Game|GetPlayerCharacter 0)))
                (Input|DisableInput _asfirst_person_character_bp_3 (Game|GetPlayerController 0))
                (Viewport|RemoveAllWidgets)
                (bind _returnvalue_5 (UserInterface|CreateWidget "/Game/BPs/Laser/DeathByLaser_WB.DeathByLaser_WB_C"))
                (UserInterface|Viewport|AddtoViewport _returnvalue_5 0)
                (Utilities|Time|PauseTimerbyHandle (Variables|Default|GetTimerHandle))
                (CameraFades|StartCameraFade :self (Game|GetPlayerCameraManager 0) :ToAlpha 1.0 :Duration 1.0 :bHoldWhenFinished true)
                (Utilities|FlowControl|Delay 2.0)
                (CameraFades|StartCameraFade :self (Game|GetPlayerCameraManager 0) :FromAlpha 1.0 :Duration 1.0 :bHoldWhenFinished true)
                (Widget|RemovefromParent _returnvalue_5)
                (Actor|DestroyActor _asfirst_person_character_bp_3)
                (goto _label_2 Reset))))
          (else
            ;[1 1 1] LineTrace ignores cube
            (bind _outhit_2 (Collision|LineTraceForObjects (Transformation|GetWorldLocation (Variables|Default|GetLaserStartPoint)) (Transformation|GetActorLocation (.AsFirst%20Person%20Character%20BP (Utilities|Casting|CastToFirstPersonCharacter_BP (Game|GetPlayerCharacter 0)))) (Variables|Default|GetObjectTypes) false (Utilities|Array|MakeArray _cube) "None"))
            (Transformation|SetWorldLocation (Variables|Default|GetSparks) (.Location (Collision|BreakHitResult _outhit_2)) false false)
            (Transformation|SetWorldLocation (Variables|Default|GetSparksSound) (.Location (Collision|BreakHitResult _outhit_2)) false false)
            (Class|ParticleSystemComponent|SetBeamEndPoint (Variables|Default|GetLaserBeam) 0 (.Location (Collision|BreakHitResult _outhit_2)))
            (if (== (.HitActor (Collision|BreakHitResult _outhit_2)) _asfirst_person_character_bp)
              (goto _label_2))))
        (else
          (goto _label))))
    (:then_1
      ;[1 1 1] Cooldown functionality
      (Utilities|FlowControl|DoOnce false :!label _label_3
        (:Completed
          (Default|SecondsBeforeDeactivation (Variables|Default|GetLaserAttackWidget))
          (Utilities|FlowControl|Delay (Variables|Default|GetSecondsBeforeDeactivation))
          (Utilities|Time|PauseTimerbyHandle (Variables|Default|GetTimerHandle))
          (Rendering|SetVisibility (Variables|Default|GetSparks) false false)
          (Rendering|SetVisibility (Variables|Default|GetLaserBeam) false false)
          (Class|AudioComponent|SetPaused (Variables|Default|GetSparksSound) true)
          (if (Variables|Default|GetStop?)
            _
            (else
              (Default|SecondsBeforeActivation (Variables|Default|GetLaserAttackWidget))
              (Utilities|FlowControl|Delay (Variables|Default|GetSecondsBeforeActivation))
              (if (Variables|Default|GetStop?)
                _
                (else
                  (Utilities|Time|UnpauseTimerbyHandle (Variables|Default|GetTimerHandle))
                  (Rendering|SetVisibility (Variables|Default|GetSparks) true false)
                  (Rendering|SetVisibility (Variables|Default|GetLaserBeam) true false)
                  (Class|AudioComponent|SetPaused (Variables|Default|GetSparksSound) false)
                  (goto _label_3 Reset)))))
          (Variables|Default|SetStop? false)
          (goto _label_3 Reset))))))

(event Custom|BeginPlay
  (bind _returnvalue (Game|GetPlayerCharacter 0))
  (bind _asfirst_person_character_bp (Utilities|Casting|CastToFirstPersonCharacter_BP _returnvalue))
  (bind _returnvalue_2 (Transformation|GetActorLocation _asfirst_person_character_bp))
  ;[1 1 1] Create Beam
  (if (Variables|Default|GetisRed?)
    (bind _returnvalue_3 (UserInterface|CreateWidget "/Game/BPs/Laser/LaserAttackingBP/Sensed_Red.Sensed_Red_C"))
    (bind _output_get (Variables|Default|SetSensedWidgetRed _returnvalue_3))
    (UserInterface|Viewport|AddtoViewport _output_get 0)
    (else
      (bind _returnvalue_4 (UserInterface|CreateWidget "/Game/BPs/Laser/LaserAttackingBP/Sensed_Blue.Sensed_Blue_C"))
      (bind _output_get_2 (Variables|Default|SetSensedWidgetBlue _returnvalue_4))
      (UserInterface|Viewport|AddtoViewport _output_get_2 0)))
  (Utilities|IsValid (Variables|Default|GetSensedWidgetRed)
    (:Is%20Valid
      (Utilities|FlowControl|Sequence
        (:then_0
          (Utilities|FlowControl|Delay 1.5)
          (Widget|RemovefromParent (Variables|Default|GetSensedWidgetRed)))
        (:then_1
          ;;[1 1 1] Widget
          (bind _returnvalue_5 (UserInterface|CreateWidget "/Game/BPs/Laser/LaserAttackingBP/LaserAttackWidget.LaserAttackWidget_C" :!label _label))
          (bind _output_get_3 (Variables|Default|SetLaserAttackWidget _returnvalue_5))
          (UserInterface|Viewport|AddtoViewport _output_get_3 0)
          (bind _output_get_4 (Variables|/Game/BPs/Laser/LaserAttackingBP/LaserAttackWidget.LaserAttackWidget_C|SetSecondsBeforeActivationWidget _output_get_3 (Variables|Default|GetSecondsBeforeActivation)))
          (Default|SecondsBeforeActivation _output_get_3)
          (Variables|/Game/BPs/Laser/LaserAttackingBP/LaserAttackWidget.LaserAttackWidget_C|SetSecondsBeforeDeactivationWidget _output_get_3 (Variables|Default|GetSecondsBeforeDeactivation))
          (Utilities|FlowControl|Delay _output_get_4)
          (if (Variables|Default|GetStop?)
            (Variables|Default|SetStop? false)
            (else
              (bind _returnvalue_6 (Collision|LineTraceForObjects (Transformation|GetWorldLocation (Variables|Default|GetLaserStartPoint)) _returnvalue_2 (Variables|Default|GetObjectTypes) false 0 "None"))
              (if _returnvalue_6
                (CallFunction|CreateBeam (Transformation|GetWorldLocation (Variables|Default|GetLaserStartPoint)) _returnvalue_2)
                (if (Variables|Default|GetisRed?)
                  (CallFunction|SetMaterial/Sparks/SparksSoundRed)
                  (else
                    (CallFunction|SetMaterial/Sparks/SparksSoundBlue)))
                (bind _returnvalue_7 (Utilities|Time|SetTimerbyEvent (EventDispatchers|CreateEvent :!event Custom|LookIfCubeCollides) 0.05 true))
                (Variables|Default|SetTimerHandle _returnvalue_7)))))))
    (:Is%20Not%20Valid
      (Utilities|FlowControl|Sequence
        (:then_0
          (goto _label))
        (:then_1
          (Utilities|FlowControl|Delay 1.5)
          (Widget|RemovefromParent (Variables|Default|GetSensedWidgetBlue)))))))

(event EventBeginPlay
  (bind _staticmesh (Variables|Default|GetStaticMesh))
  ;[1 1 1] Create Beam
  (bind _returnvalue (Rendering|Material|CreateDynamicMaterialInstance _staticmesh 0 "/Game/BPs/PuzzleStuff/Platforms/PlatformMat_Inst.PlatformMat_Inst" "None" :!class /Script/Engine.PrimitiveComponent))
  (bind _output_get (Variables|Default|SetMaterialCubeLaser _returnvalue))
  (Rendering|Material|SetMaterial _staticmesh 0 _output_get)
  (if (not (Variables|Default|GetisRed?))
    (Rendering|Material|SetVectorParameterValue (Variables|Default|GetMaterialCubeLaser) "Color" "(R=0.000000,G=0.000000,B=1.000000,A=1.000000)" :!class /Script/Engine.MaterialInstanceDynamic)))

(fn ConstructionScript)

(fn CreateBeam
  (params (StartPoint :type Vector) (EndPoint :type Vector))
  (bind _returnvalue (Effects|SpawnEmitteratLocation "/Game/BPs/Laser/LaserParticle/Laser_P.Laser_P" StartPoint))
  (bind _output_get (Variables|Default|SetLaserBeam _returnvalue))
  (Class|ParticleSystemComponent|SetBeamEndPoint _output_get 0 EndPoint))

(fn SetMaterial/Sparks/SparksSoundRed
  (bind _returnvalue (Game|GetPlayerCharacter 0))
  (bind _asfirst_person_character_bp (Utilities|Casting|CastToFirstPersonCharacter_BP _returnvalue))
  (bind _returnvalue_2 (Transformation|GetActorLocation _asfirst_person_character_bp))
  (bind _returnvalue_3 (Rendering|Material|CreateDynamicMaterialInstance "/Game/BPs/Laser/LaserParticle/LaserMaterial_Inst.LaserMaterial_Inst" "None" :!class /Script/Engine.KismetMaterialLibrary))
  (bind _output_get (Variables|Default|SetMaterialRef _returnvalue_3))
  (Rendering|Material|SetMaterial (Variables|Default|GetLaserBeam) 0 _output_get)
  (Rendering|Material|SetVectorParameterValue _output_get "EmissiveColour" "(R=1.000000,G=0.000000,B=0.000000,A=1.000000)" :!class /Script/Engine.MaterialInstanceDynamic)
  (bind _returnvalue_4 (Effects|SpawnEmitteratLocation "/Game/BPs/Laser/Sparks/P_WeldSparks_Red.P_WeldSparks_Red" _returnvalue_2))
  (Variables|Default|SetSparks _returnvalue_4)
  (bind _returnvalue_5 (Audio|SpawnSoundatLocation "/Game/BPs/Laser/Sparks/CubeSparksEffect.CubeSparksEffect" _returnvalue_2 "0, 0, 0" 1.0 1.0 0.0 (Variables|Default|GetAttenuationSparks) 0))
  (Variables|Default|SetSparksSound _returnvalue_5))

(fn SetMaterial/Sparks/SparksSoundBlue
  (bind _returnvalue (Game|GetPlayerCharacter 0))
  (bind _asfirst_person_character_bp (Utilities|Casting|CastToFirstPersonCharacter_BP _returnvalue))
  (bind _returnvalue_2 (Transformation|GetActorLocation _asfirst_person_character_bp))
  (bind _returnvalue_3 (Rendering|Material|CreateDynamicMaterialInstance "/Game/BPs/Laser/LaserParticle/LaserMaterial_Inst.LaserMaterial_Inst" "None" :!class /Script/Engine.KismetMaterialLibrary))
  (bind _output_get (Variables|Default|SetMaterialRef _returnvalue_3))
  (Rendering|Material|SetMaterial (Variables|Default|GetLaserBeam) 0 _output_get)
  (Rendering|Material|SetVectorParameterValue _output_get "EmissiveColour" "(R=0.000000,G=0.000000,B=1.000000,A=1.000000)" :!class /Script/Engine.MaterialInstanceDynamic)
  (bind _returnvalue_4 (Effects|SpawnEmitteratLocation "/Game/BPs/Laser/Sparks/P_WeldSparks_Blue.P_WeldSparks_Blue" _returnvalue_2))
  (Variables|Default|SetSparks _returnvalue_4)
  (bind _returnvalue_5 (Audio|SpawnSoundatLocation "/Game/BPs/Laser/Sparks/CubeSparksEffect.CubeSparksEffect" _returnvalue_2 "0, 0, 0" 1.0 1.0 0.0 (Variables|Default|GetAttenuationSparks) 0))
  (Variables|Default|SetSparksSound _returnvalue_5))