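; Level actor that builds a yellow paintable floor at BeginPlay by spawning a grid of CubePintableYellow_BP cubes from its root location.
; Each cube's LeftLocation places the next cube along a row, while a FrontLocation starts the following row.
; A DoOnce captures the first cube's front, then each row-starting cube supplies the next.
; Redraw calls itself until the counter passes Column, with Row setting row length.
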(event Custom|Redraw
  (for _index (range 0 (Variables|Default|GetRow))
    (bind _returnvalue (Game|SpawnActorfromClass "/Game/Levels/Rooms/Level5/Pintable_Floor/YellowFloor/CubePintableYellow_BP.CubePintableYellow_BP_C" (Math|Transform|MakeTransform (Variables|Default|GetNext) "0, 0, 0" (Variables|Default|GetScale)) "Undefined" 0 0))
    (Variables|Default|SetNext (Variables|/Game/Levels/Rooms/Level5/Pintable_Floor/YellowFloor/CubePintableYellow_BP.CubePintableYellow_BP_C|GetLeft_Location _returnvalue))
    (Utilities|FlowControl|DoOnce false
      (:Completed
        (Variables|Default|SetFront (Variables|/Game/Levels/Rooms/Level5/Pintable_Floor/YellowFloor/CubePintableYellow_BP.CubePintableYellow_BP_C|GetFront_Location _returnvalue)))))
  (bind _returnvalue_2 (Game|SpawnActorfromClass "/Game/Levels/Rooms/Level5/Pintable_Floor/YellowFloor/CubePintableYellow_BP.CubePintableYellow_BP_C" (Math|Transform|MakeTransform (Variables|Default|GetFront) "0, 0, 0" (Variables|Default|GetScale)) "Undefined" 0 0))
  (Variables|Default|SetNext (Variables|/Game/Levels/Rooms/Level5/Pintable_Floor/YellowFloor/CubePintableYellow_BP.CubePintableYellow_BP_C|GetLeft_Location _returnvalue_2))
  (Variables|Default|SetFront (Variables|/Game/Levels/Rooms/Level5/Pintable_Floor/YellowFloor/CubePintableYellow_BP.CubePintableYellow_BP_C|GetFront_Location _returnvalue_2))
  (if (<= (Variables|Default|GetCount) (Variables|Default|GetColumn))
    (Variables|Default|SetCount (+ (Variables|Default|GetCount) 1))
    (CallFunction|Redraw)))

(event EventBeginPlay
  (Variables|Default|SetNext (Transformation|GetWorldLocation (Variables|Default|GetDefaultSceneRoot)))
  (for _index (range 0 (Variables|Default|GetRow))
    (bind _returnvalue (Game|SpawnActorfromClass "/Game/Levels/Rooms/Level5/Pintable_Floor/YellowFloor/CubePintableYellow_BP.CubePintableYellow_BP_C" (Math|Transform|MakeTransform (Variables|Default|GetNext) "0, 0, 0" (Variables|Default|GetScale)) "Undefined" 0 0))
    (Variables|Default|SetNext (Variables|/Game/Levels/Rooms/Level5/Pintable_Floor/YellowFloor/CubePintableYellow_BP.CubePintableYellow_BP_C|GetLeft_Location _returnvalue))
    (Utilities|FlowControl|DoOnce false
      (:Completed
        (Variables|Default|SetFront (Variables|/Game/Levels/Rooms/Level5/Pintable_Floor/YellowFloor/CubePintableYellow_BP.CubePintableYellow_BP_C|GetFront_Location _returnvalue)))))
  (bind _returnvalue_2 (Game|SpawnActorfromClass "/Game/Levels/Rooms/Level5/Pintable_Floor/YellowFloor/CubePintableYellow_BP.CubePintableYellow_BP_C" (Math|Transform|MakeTransform (Variables|Default|GetFront) "0, 0, 0" (Variables|Default|GetScale)) "Undefined" 0 0))
  (Variables|Default|SetNext (Variables|/Game/Levels/Rooms/Level5/Pintable_Floor/YellowFloor/CubePintableYellow_BP.CubePintableYellow_BP_C|GetLeft_Location _returnvalue_2))
  (Variables|Default|SetFront (Variables|/Game/Levels/Rooms/Level5/Pintable_Floor/YellowFloor/CubePintableYellow_BP.CubePintableYellow_BP_C|GetFront_Location _returnvalue_2))
  (if (<= (Variables|Default|GetCount) (Variables|Default|GetColumn))
    (Variables|Default|SetCount (+ (Variables|Default|GetCount) 1))
    (CallFunction|Redraw)))

(fn ConstructionScript)