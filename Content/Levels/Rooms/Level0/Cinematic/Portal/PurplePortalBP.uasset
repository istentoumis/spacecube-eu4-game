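; Purple portal actor for a Level0 cinematic that fades in and can launch thunder balls.
; On BeginPlay, parallel timelines animate Fade and Density on a dynamic material instance from its particle system.
; If ShouldSpawn is set, it spawns a ThunderBallBP at its arrow, then replaces it after a delay, leaving the portal open.
; Otherwise, after a delay, Opposite reverses Density then Fade and destroys the portal.
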(event Custom|Opposite
  (bind _materialref (Variables|Default|GetMaterialRef))
  (bind _fade (Timeline|Timeline_1 Play)
    (:Update
      (Rendering|Material|SetScalarParameterValue _materialref "Density" (Math|Float|Lerp 7.0 0.0 _fade) :!class /Script/Engine.MaterialInstanceDynamic))
    (:Finished
      (bind _fade_2 (Timeline|Timeline_0 Play) ; FadePortal
        (:Update
          (Rendering|Material|SetScalarParameterValue _materialref "Fade" (Math|Float|Lerp 0.0 -1.0 _fade_2) :!class /Script/Engine.MaterialInstanceDynamic))
        (:Finished
          (Actor|DestroyActor))))))

(event EventBeginPlay
  (bind _arrow (Variables|Default|GetArrow))
  (bind _returnvalue (Transformation|GetWorldLocation _arrow))
  (bind _returnvalue_2 (Transformation|GetWorldRotation _arrow))
  (bind _returnvalue_3 (Math|Transform|MakeTransform _returnvalue _returnvalue_2 "0.500000,0.500000,0.500000"))
  (bind _returnvalue_4 (Rendering|Material|CreateDynamicMaterialInstance (Variables|Default|GetParticleSystem) 0 "/Game/Levels/Rooms/Level0/Cinematic/Portal/Material/M_PortalPurple_Inst.M_PortalPurple_Inst" "None" :!class /Script/Engine.PrimitiveComponent))
  (bind _output_get (Variables|Default|SetMaterialRef _returnvalue_4))
  (Utilities|FlowControl|Sequence
    (:then_0
      (bind _fade (Timeline|FadePortal Play) ; FadePortal
        (:Update
          (Rendering|Material|SetScalarParameterValue _output_get "Fade" (Math|Float|Lerp -1.0 0.0 _fade) :!class /Script/Engine.MaterialInstanceDynamic))))
    (:then_1
      (bind _fade_2 (Timeline|FadeDensity Play)
        (:Update
          (Rendering|Material|SetScalarParameterValue _output_get "Density" (Math|Float|Lerp 0.0 7.0 _fade_2) :!class /Script/Engine.MaterialInstanceDynamic))
        (:Finished
          (if (Variables|Default|GetShouldSpawn?)
            (bind _returnvalue_5 (Game|SpawnActorfromClass "/Game/Levels/Rooms/Level0/Cinematic/Portal/ThunderBall/ThunderBallBP.ThunderBallBP_C" _returnvalue_3 "Undefined" 0 0))
            (Utilities|FlowControl|Delay 2.0)
            (Actor|DestroyActor _returnvalue_5)
            (Game|SpawnActorfromClass "/Game/Levels/Rooms/Level0/Cinematic/Portal/ThunderBall/ThunderBallBP.ThunderBallBP_C" _returnvalue_3 "Undefined" 0 0)
            (else
              (Utilities|FlowControl|Delay 2.0)
              (CallFunction|Opposite))))))))

(fn ConstructionScript)