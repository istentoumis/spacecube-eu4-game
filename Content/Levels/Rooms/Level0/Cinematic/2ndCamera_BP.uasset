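; 2ndCamera_BP is a cinematic camera actor in the Level0 room that performs a delayed dolly move.
; Twenty seconds after BeginPlay, the MoveCamera timeline drives the camera component along its relative X axis, scaled by MovementSpeed.
; A RotateCamera timeline that would pitch the camera after its own delay is present but disconnected, so it never runs.
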(event EventBeginPlay
  (Utilities|FlowControl|Delay 2e+01)
  (Utilities|FlowControl|Sequence
    (:then_0
      (bind _newtrack_0 (Timeline|MoveCamera Play)
        (:Update
          (Transformation|SetRelativeLocation (Variables|CameraActor|GetCameraComponent) (Math|Vector|MakeVector (* _newtrack_0 (Variables|Default|GetMovementSpeed)) 0.0 0.0) false false))))))

(fn ConstructionScript)